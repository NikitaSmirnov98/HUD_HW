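; BP_Shape is a falling collectible shape that the player catches in the Geometry Catcher game.
; Each tick it moves down by FallSpeed using a swept world offset.
; On overlapping BP_Player it destroys itself, plays a click sound and tells GameManager to increment both the total and the per-color collected counts, keyed by ColorIndex.
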(event EventBeginPlay)

(event Collision|EventActorBeginOverlap
  (params (OtherActor :type Actor%20Object%20Reference))
  ;[1 1 1] When shape overlaps with player - destroy it and increase score.
  (Utilities|Casting|CastToBP_Player OtherActor)
  (Actor|DestroyActor)
  (Audio|SpawnSound2D "/Engine/VREditor/Sounds/UI/Click_on_Button_Cue.Click_on_Button_Cue" 1.0 1.0 0.0 0)
  (Default|IncrementShapesCollected (Variables|Default|GetGameManager))
  (Default|IncrementColoredShapesCollected (Variables|Default|GetGameManager) (Variables|Default|GetColorIndex)))

(event EventTick
  (params (DeltaSeconds :type Float%20%28single-precision%29))
  ;[1 1 1] Making shapes move
  (Transformation|AddActorWorldOffset (Math|Vector|MakeVector 0.0 0.0 (* (* DeltaSeconds (Variables|Default|GetFallSpeed)) -1.0)) true))

(fn ConstructionScript)